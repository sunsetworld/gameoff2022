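; Player Character Blueprint handling camera-relative movement, jump, sprint, light toggle, pause menu and health, with death destroying the actor.
; Timelines animate the forward spring arm's length to switch between first and third person, while BackwardMode selects which spring arm receives camera pitch.
; Fall damage uses retriggerable delays to set TempDamage during long falls, applies it on landing through AnyDamage, and never resets it.
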(event EventBeginPlay
  (Variables|Default|SetJumpMaxHoldTime (Variables|Default|GetjumpTime))
  (Rendering|ToggleVisibility (Variables|Default|GetPointLight) false)
  (Variables|Default|SetoriginalWalkSpeed (Variables|/Script/Engine.CharacterMovementComponent|GetMaxWalkSpeed (Variables|Character|GetCharacterMovement))))

(event Collision|EventActorBeginOverlap
  (params (OtherActor :type Actor%20Object%20Reference)))

(event EventTick
  (params (DeltaSeconds :type Float%20%28single-precision%29)))

(event Game|Damage|EventAnyDamage
  (params (Damage :type Float%20%28single-precision%29) (DamageType :type Damage%20Type%20Object%20Reference) (InstigatedBy :type Controller%20Object%20Reference) (DamageCauser :type Actor%20Object%20Reference))
  ;[1 1 1] Kill
  (Variables|Default|Sethealth (- (Variables|Default|Gethealth) Damage))
  (if (<= (Variables|Default|Gethealth) 0.0)
    (Audio|PlaySoundatLocation "/Game/Sounds/kenney_digitalaudio/Audio/zapThreeToneDown.zapThreeToneDown" (Transformation|GetActorLocation) "0, 0, 0" 1.0 1.0 0.0 0 0 0 0)
    (Game|Feedback|ClientPlayForceFeedback (Game|GetPlayerController 0) "/Game/Misc/FF03.FF03" "Kill" false false false)
    (Actor|DestroyActor)))

(event EventOnMovementModeChanged
  (params (PrevMovementMode :type EMovementMode%20Enum :default "MOVE_None") (NewMovementMode :type EMovementMode%20Enum :default "MOVE_None") (PrevCustomMode :type Byte :default 0) (NewCustomMode :type Byte :default 0))
  (bind _charactermovement (Variables|Character|GetCharacterMovement))
  (bind _returnvalue (AI|Components|NavMovement|IsFalling _charactermovement))
  ;[1 1 1] Fall Damage
  (if (Utilities|Enum|Equal(Enum) NewMovementMode "MOVE_Falling")
    (Utilities|FlowControl|RetriggerableDelay 1.6)
    (if _returnvalue
      (Variables|Default|SettempDamage 1e+02)
      (Utilities|FlowControl|RetriggerableDelay 1.0)
      (if _returnvalue
        (Variables|Default|SettempDamage 1e+02)))))

(event EventOnLanded
  (params (Hit :type Hit%20Result%20Structure%20%28by%20ref%29))
  ;[1 1 1] Fall Damage
  (Game|Damage|ApplyDamage self (Variables|Default|GettempDamage) 0 0))

(event Input|ActionEvents|InputActionJump
  (params (Key :type Key%20Structure :default "None"))
  ;[1 1 1] Player Jump
  (:Pressed
    (Character|Jump)
    (Audio|PlaySound2D "/Game/Sounds/kenney_digitalaudio/Audio/phaseJump1.phaseJump1" 1.0 1.0 0.0 0 0)
    (Game|Feedback|ClientPlayForceFeedback (Game|GetPlayerController 0) "/Game/Misc/FF01.FF01" "Jump" false false false)))

(event Input|ActionEvents|InputActionFPSKey
  (params (Key :type Key%20Structure :default "None"))
  ;[1 1 1] First Person Toggle
  (:Pressed
    (Utilities|FlowControl|FlipFlop
      (:A
        (Audio|PlaySoundatLocation "/Game/Sounds/kenney_digitalaudio/Audio/threeTone1.threeTone1" (Transformation|GetActorLocation) "0, 0, 0" 1.0 1.0 0.0 0 0 0 0)
        (bind _thirdtofirst (Timeline|CamChange PlayFromStart)
          (:Update
            (Variables|/Script/Engine.SpringArmComponent|SetTargetArmLength (Variables|Default|GetFwdSpringArm) _thirdtofirst)
            (Variables|Default|SetfirstPersonMode true))))
      (:B
        (Audio|PlaySoundatLocation "/Game/Sounds/kenney_digitalaudio/Audio/threeTone2.threeTone2" (Transformation|GetActorLocation) "0, 0, 0" 1.0 1.0 0.0 0 0 0 0)
        (bind _firsttothird (Timeline|Timeline_0 PlayFromStart)
          (:Update
            (Variables|/Script/Engine.SpringArmComponent|SetTargetArmLength (Variables|Default|GetFwdSpringArm) _firsttothird)
            (Variables|Default|SetfirstPersonMode false)))))))

(event Input|ActionEvents|InputActionMuteToggle
  (params (Key :type Key%20Structure :default "None")))

(event Input|ActionEvents|InputActionLightToggle
  (params (Key :type Key%20Structure :default "None"))
  (:Pressed
    (Rendering|ToggleVisibility (Variables|Default|GetPointLight) false)))

(event Input|ActionEvents|InputActionPauseToggle
  (params (Key :type Key%20Structure :default "None"))
  (bind _returnvalue (Game|Player|GetPlayerPawn 0))
  (bind _playerstate (Variables|/Script/Engine.Pawn|GetPlayerState _returnvalue))
  (bind _returnvalue_2 (Game|GetPlayerController _playerstate))
  ;[1 1 1] Pause Game
  (:Pressed
    (Utilities|FlowControl|FlipFlop
      (:A
        (bind _returnvalue_3 (UserInterface|CreateWidget "/Game/Blueprints/Widgets/BP_PauseWidget.BP_PauseWidget_C"))
        (UserInterface|Viewport|AddtoViewport _returnvalue_3 0)
        (Game|SetGamePaused true)
        (Variables|/Script/Engine.PlayerController|SetbShowMouseCursor _returnvalue_2 true))
      (:B
        (Widget|RemovefromParent _returnvalue_3)
        (Game|SetGamePaused false)
        (Variables|/Script/Engine.PlayerController|SetbShowMouseCursor _returnvalue_2 false)))))

(event Input|ActionEvents|InputActionSprintToggle
  (params (Key :type Key%20Structure :default "None"))
  ;[1 1 1] Sprint
  (:Pressed
    (bind _output_get (Variables|/Script/Engine.CharacterMovementComponent|SetMaxWalkSpeed (Variables|Character|GetCharacterMovement) (* (Variables|Default|GetoriginalWalkSpeed) (Variables|Default|GetsprintMultiplier))))
    (Development|PrintString (Utilities|String|ToString(Float) _output_get)))
  (:Released
    (Variables|/Script/Engine.CharacterMovementComponent|SetMaxWalkSpeed (Variables|Character|GetCharacterMovement) (Variables|Default|GetoriginalWalkSpeed))))

(event Input|ActionEvents|InputActionBoxToggle
  (params (Key :type Key%20Structure :default "None")))

(event Input|AxisEvents|InputAxisCam_Up/Down
  (params (AxisValue :type Float%20%28single-precision%29))
  ;[1 1 1] Move Camera
  (if (not (Variables|Default|GetBackwardMode))
    (Transformation|AddRelativeRotation (Variables|Default|GetFwdSpringArm) (Math|Rotator|MakeRotator 0.0 AxisValue 0.0) false false)
    (else
      (Transformation|AddRelativeRotation (Variables|Default|GetBkdSpringArm) (Math|Rotator|MakeRotator 0.0 AxisValue 0.0) false false))))

(event Input|AxisEvents|InputAxisPlayer_Up/Down
  (params (AxisValue :type Float%20%28single-precision%29))
  ;[1 1 1] Player Move
  (Pawn|Input|AddMovementInput (Math|Vector|GetForwardVector (Math|Rotator|MakeRotator 0.0 0.0 (.Yaw (Math|Rotator|BreakRotator (Pawn|GetControlRotation :!class /Script/Engine.Pawn))))) AxisValue false))

(event Input|AxisEvents|InputAxisPlayer_Left/Right
  (params (AxisValue :type Float%20%28single-precision%29))
  ;[1 1 1] Player Move
  (Pawn|Input|AddMovementInput (Math|Vector|GetRightVector (Math|Rotator|MakeRotator 0.0 0.0 (.Yaw (Math|Rotator|BreakRotator (Pawn|GetControlRotation :!class /Script/Engine.Pawn))))) AxisValue false))

(event Input|AxisEvents|InputAxisCam_Left/Right
  (params (AxisValue :type Float%20%28single-precision%29))
  ;[1 1 1] Rotate Player
  (Pawn|Input|AddControllerYawInput AxisValue))

(fn ConstructionScript)