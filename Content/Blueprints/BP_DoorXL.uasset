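; BP_DoorXL is a two-part door that opens when the player walks into its trigger.
; An EnterTrigger overlap passing the BP_Player cast snaps DoorL and DoorR0 to the same fixed world rotation, with no animation or closing logic.
; A SoundHasPlayed flag limits the opening sound at the actor's location to the first entry.
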(event OnComponentBeginOverlap(EnterTrigger)
  (params (OverlappedComponent :type Primitive%20Component%20Object%20Reference) (OtherActor :type Actor%20Object%20Reference) (OtherComp :type Primitive%20Component%20Object%20Reference) (OtherBodyIndex :type Integer) (bFromSweep :type Boolean) (SweepResult :type Hit%20Result%20Structure%20%28by%20ref%29))
  (Utilities|Casting|CastToBP_Player OtherActor)
  (Transformation|SetWorldRotation (Variables|Default|GetdoorL) "0,-90.000000, 0" false false)
  (Transformation|SetWorldRotation (Variables|Default|GetDoorR_0) "0,-90.000000, 0" false false)
  (if (not (Variables|Default|GetsoundHasPlayed))
    (Audio|PlaySoundatLocation "/Game/Sounds/kenney_rpgaudio/Audio/doorOpen_1.doorOpen_1" (Transformation|GetActorLocation) "0, 0, 0" 1.0 1.0 0.0 0 0 0 0)
    (Variables|Default|SetsoundHasPlayed true)))

(event EventBeginPlay)

(event Collision|EventActorBeginOverlap
  (params (OtherActor :type Actor%20Object%20Reference)))

(event EventTick
  (params (DeltaSeconds :type Float%20%28single-precision%29)))

(fn ConstructionScript)