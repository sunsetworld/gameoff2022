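; BP_Fire is a fire effect actor with a particle system, a flickering point light and sound.
; On BeginPlay it plays a fire sound at its box and starts the FlickerTime timeline.
; Timeline updates set light intensity to a random target re-rolled after short random delays, with Lerp alpha fixed at 1, so it snaps.
; DeactivateFire deactivates the particles and light but leaves the sound untouched.
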(event EventBeginPlay
  (bind _pointlight (Variables|Default|GetPointLight))
  (Audio|PlaySoundatLocation "/Game/StarterContent/Audio/Fire01.Fire01" (Transformation|GetWorldLocation (Variables|Default|GetBox)) "0, 0, 0" 1.0 1.0 0.0 0 0 0 0)
  (Timeline|FlickerTime Play
    (:Update
      (Utilities|FlowControl|Sequence
        (:then_0
          (Rendering|Components|Light|SetIntensity _pointlight (Math|Float|Lerp (Variables|/Script/Engine.LightComponentBase|GetIntensity _pointlight) (Variables|Default|GettargetIntensity) 1.0)))
        (:then_1
          (Utilities|FlowControl|Delay (Math|Random|RandomFloatinRange 0.01 0.05))
          (Variables|Default|SettargetIntensity (Math|Random|RandomFloatinRange 1e+03 1e+05)))))))

(event Collision|EventActorBeginOverlap
  (params (OtherActor :type Actor%20Object%20Reference)))

(event EventTick
  (params (DeltaSeconds :type Float%20%28single-precision%29)))

(fn ConstructionScript)

(fn DeactivateFire
  (Components|Activation|Deactivate (Variables|Default|GetFireSystem))
  (Components|Activation|Deactivate (Variables|Default|GetPointLight)))