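; BP_Enemy is an enemy that chases the player and can either hurt them or be destroyed for points.
; PawnSensing spots BP_Player and triggers AIMoveTo toward that actor.
; Overlap with KillColl applies DamAmount damage to the player and destroys the enemy.
; Overlap with JumpCollision, apparently a stomp zone, adds ScoreIncrement to the player's Score and destroys the enemy.
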(event OnSeePawn(PawnSensing)
  (params (Pawn :type Pawn%20Object%20Reference))
  (bind _asbp_player (Utilities|Casting|CastToBP_Player Pawn))
  (AI|AIMoveTo self (Transformation|GetActorLocation _asbp_player) _asbp_player 5.0 false))

(event OnComponentBeginOverlap(KillColl)
  (params (OverlappedComponent :type Primitive%20Component%20Object%20Reference) (OtherActor :type Actor%20Object%20Reference) (OtherComp :type Primitive%20Component%20Object%20Reference) (OtherBodyIndex :type Integer) (bFromSweep :type Boolean) (SweepResult :type Hit%20Result%20Structure%20%28by%20ref%29))
  (bind _asbp_player (Utilities|Casting|CastToBP_Player OtherActor))
  (Game|Damage|ApplyDamage _asbp_player (Variables|Default|GetdamAmount) 0 0)
  (Actor|DestroyActor))

(event OnComponentBeginOverlap(JumpCollision)
  (params (OverlappedComponent :type Primitive%20Component%20Object%20Reference) (OtherActor :type Actor%20Object%20Reference) (OtherComp :type Primitive%20Component%20Object%20Reference) (OtherBodyIndex :type Integer) (bFromSweep :type Boolean) (SweepResult :type Hit%20Result%20Structure%20%28by%20ref%29))
  (bind _asbp_player (Utilities|Casting|CastToBP_Player OtherActor))
  (Variables|/Game/Blueprints/BP_Player.BP_Player_C|Setscore _asbp_player (+ (Variables|/Game/Blueprints/BP_Player.BP_Player_C|Getscore _asbp_player) (Variables|Default|GetscoreIncrement)))
  (Actor|DestroyActor))

(event EventBeginPlay)

(event Collision|EventActorBeginOverlap
  (params (OtherActor :type Actor%20Object%20Reference)))

(fn ConstructionScript)