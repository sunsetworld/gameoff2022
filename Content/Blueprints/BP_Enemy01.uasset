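; BP_Enemy01 is a simple enemy that chases the player, hurts them on contact and can be killed through a separate jump hitbox.
; PawnSensing spots BP_Player and issues an AI MoveTo toward it.
; A MainCollision overlap with the player applies DamAmount damage and destroys the enemy.
; A JumpCollision overlap with the player destroys the enemy without dealing damage.
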(event OnComponentBeginOverlap(EnemyMesh)
  (params (OverlappedComponent :type Primitive%20Component%20Object%20Reference) (OtherActor :type Actor%20Object%20Reference) (OtherComp :type Primitive%20Component%20Object%20Reference) (OtherBodyIndex :type Integer) (bFromSweep :type Boolean) (SweepResult :type Hit%20Result%20Structure%20%28by%20ref%29)))

(event OnComponentBeginOverlap(MainCollision)
  (params (OverlappedComponent :type Primitive%20Component%20Object%20Reference) (OtherActor :type Actor%20Object%20Reference) (OtherComp :type Primitive%20Component%20Object%20Reference) (OtherBodyIndex :type Integer) (bFromSweep :type Boolean) (SweepResult :type Hit%20Result%20Structure%20%28by%20ref%29))
  (bind _asbp_player (Utilities|Casting|CastToBP_Player OtherActor))
  (CallFunction|DamagePlayer _asbp_player))

(event OnComponentBeginOverlap(JumpCollision)
  (params (OverlappedComponent :type Primitive%20Component%20Object%20Reference) (OtherActor :type Actor%20Object%20Reference) (OtherComp :type Primitive%20Component%20Object%20Reference) (OtherBodyIndex :type Integer) (bFromSweep :type Boolean) (SweepResult :type Hit%20Result%20Structure%20%28by%20ref%29))
  (Utilities|Casting|CastToBP_Player OtherActor)
  (Actor|DestroyActor))

(event OnSeePawn(PawnSensing)
  (params (Pawn :type Pawn%20Object%20Reference))
  (bind _asbp_player (Utilities|Casting|CastToBP_Player Pawn))
  (AI|AIMoveTo (AI|GetAIController 0) "0, 0, 0" _asbp_player -1.0 "Default" "Default" true true))

(event EventBeginPlay)

(event Collision|EventActorBeginOverlap
  (params (OtherActor :type Actor%20Object%20Reference)))

(event EventTick
  (params (DeltaSeconds :type Float%20%28single-precision%29)))

(fn ConstructionScript)

(fn DamagePlayer
  (params (DamagedActor :type Actor%20Object%20Reference))
  (Game|Damage|ApplyDamage DamagedActor (Variables|Default|GetdamAmount) 0 0)
  (Actor|DestroyActor))